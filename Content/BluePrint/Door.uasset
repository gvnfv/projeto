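; Double sliding door that the player opens and closes by interacting inside its trigger box, with opening gated on HasKey.
; The box overlap registers the door as BP_ThirdPersonCharacter's LastInteractObject and toggles CanInteract.
; Interact uses a FlipFlop to play or reverse two timelines sliding DoorR and DoorL along relative X, updating DoorOpen when the right one finishes.
; The FlipFlop advances even when HasKey is false.
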(event OnComponentBeginOverlap(Box)
  (params (OverlappedComponent :type Primitive%20Component%20Object%20Reference) (OtherActor :type Actor%20Object%20Reference) (OtherComp :type Primitive%20Component%20Object%20Reference) (OtherBodyIndex :type Integer) (bFromSweep :type Boolean) (SweepResult :type Hit%20Result%20Structure%20%28by%20ref%29))
  (bind _asbp_third_person_character (Utilities|Casting|CastToBP_ThirdPersonCharacter OtherActor))
  (Variables|/Game/ThirdPerson/Blueprints/BP_ThirdPersonCharacter.BP_ThirdPersonCharacter_C|SetLastInteractObject _asbp_third_person_character self)
  (Variables|Default|SetcanInteract? true))

(event OnComponentEndOverlap(Box)
  (params (OverlappedComponent :type Primitive%20Component%20Object%20Reference) (OtherActor :type Actor%20Object%20Reference) (OtherComp :type Primitive%20Component%20Object%20Reference) (OtherBodyIndex :type Integer))
  (Utilities|Casting|CastToBP_ThirdPersonCharacter OtherActor)
  (Variables|Default|SetcanInteract? false))

(event EventInteract
  (if (Variables|Default|GetcanInteract?)
    (Utilities|FlowControl|FlipFlop
      (:A
        (if (Variables|gameplay|GetHasKey?)
          (Utilities|FlowControl|Sequence
            (:then_0
              (bind _doorr (Timeline|RDoor Play)
                (:Update
                  (Transformation|SetRelativeLocation (Variables|Default|GetDoorR) (Math|Vector|MakeVector _doorr 0.0 0.0) false false))
                (:Finished
                  (Variables|Default|SetDoorOpen? (> 0.0 _doorr)))))
            (:then_1
              (bind _doorl (Timeline|LDoor Play)
                (:Update
                  (Transformation|SetRelativeLocation (Variables|Default|GetDoorL) (Math|Vector|MakeVector _doorl 0.0 0.0) false false)))))))
      (:B
        (Utilities|FlowControl|Sequence
          (:then_0
            (Timeline|RDoor Reverse))
          (:then_1
            (Timeline|LDoor Reverse)))))))

(fn ConstructionScript)