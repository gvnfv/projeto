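; Coin pickup actor that spins continuously and can be collected by the third-person character through an interaction.
; BeginPlay rotates the mesh through a zero-delay loop, while sphere overlap registers the coin as the character's LastInteractObject and toggles CanInteract.
; Interact destroys the coin only while CanInteract is true.
; The construction script loads a data table row into Items, but the mesh assignment is disconnected and coinEvent is empty.
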(event OnComponentBeginOverlap(Sphere)
  (params (OverlappedComponent :type Primitive%20Component%20Object%20Reference) (OtherActor :type Actor%20Object%20Reference) (OtherComp :type Primitive%20Component%20Object%20Reference) (OtherBodyIndex :type Integer) (bFromSweep :type Boolean) (SweepResult :type Hit%20Result%20Structure%20%28by%20ref%29))
  (bind _asbp_third_person_character (Utilities|Casting|CastToBP_ThirdPersonCharacter OtherActor))
  (Variables|/Game/ThirdPerson/Blueprints/BP_ThirdPersonCharacter.BP_ThirdPersonCharacter_C|SetLastInteractObject _asbp_third_person_character self)
  (Variables|Default|SetCanInteract? true))

(event OnComponentEndOverlap(Sphere)
  (params (OverlappedComponent :type Primitive%20Component%20Object%20Reference) (OtherActor :type Actor%20Object%20Reference) (OtherComp :type Primitive%20Component%20Object%20Reference) (OtherBodyIndex :type Integer))
  (Utilities|Casting|CastToBP_ThirdPersonCharacter OtherActor)
  (Variables|Default|SetCanInteract? false))

(event Custom|coinEvent)

(event EventBeginPlay
  (Transformation|AddRelativeRotation (Variables|Default|GetCoin) (* "0.000000,1.000000,0.000000" 1e+01) false false :!label _label)
  (Utilities|FlowControl|Delay 0.0)
  (goto _label))

(event EventInteract
  (if (Variables|Default|GetCanInteract?)
    (Actor|DestroyActor)))

(fn ConstructionScript
  (bind _data_table_row_handle (Variables|Default|GetData%20Table%20Row%20Handle))
  (bind (_datatable _rowname) (Utilities|Struct|BreakDataTableRowHandle _data_table_row_handle))
  (bind _returnvalue (Utilities|GetDataTableRow _datatable _rowname)
    (:then
      (bind _output_get (Variables|Default|Setitems _returnvalue)))))